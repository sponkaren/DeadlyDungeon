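; Dungeon player controller that sets its starting location and rotation on BeginPlay and routes turn and info inputs.
; The Execute and Next Turn actions find the top-level turn action widgets and call their matching button-click handlers, so input shares the UI's logic.
; Right-click asks every player character to set its info if hovered.
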(event EventBeginPlay
  (Class|Controller|SetInitialLocationandRotation (Variables|Default|GetStart%20Location) (Variables|Default|GetStart%20Rotation)))

(event EventTick
  (params (DeltaSeconds :type Float%20%28single-precision%29)))

(event Input|ActionEvents|InputActionAM_Execute
  (params (Key :type Key%20Structure :default "None"))
  (:Pressed
    (bind _foundwidgets (Widget|GetAllWidgetsOfClass "/Game/Systems/UI/BP_TurnActionWidget.BP_TurnActionWidget_C" true))
    (Class|TurnActionWidget|OnExecuteButtonClicked _foundwidgets)))

(event Input|ActionEvents|InputActionAM_NextTurn
  (params (Key :type Key%20Structure :default "None"))
  (:Pressed
    (bind _foundwidgets (Widget|GetAllWidgetsOfClass "/Game/Systems/UI/BP_TurnActionWidget.BP_TurnActionWidget_C" true))
    (Class|TurnActionWidget|OnNextTurnButtonClicked _foundwidgets)))

(event Input|ActionEvents|InputActionAM_RightClick
  (params (Key :type Key%20Structure :default "None"))
  (:Pressed
    (bind _outactors (Actor|GetAllActorsOfClass "/Game/Systems/PlayerSystem/BP_PlayerCharacter.BP_PlayerCharacter_C"))
    (for _array_element _outactors
      (Default|SetInfoifHovered _array_element))))

(fn ConstructionScript)