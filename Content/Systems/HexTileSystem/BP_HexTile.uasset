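; BP_HexTile is a clickable tile actor for the hex tile system, with highlight, attack, select and attack-select overlays.
; BeginPlay hides all four overlays, and clicking the tile mesh calls HexClicked, whose logic is not defined in this graph.
; A debug label drawing the tile's name is left unconnected, and the placeholder NewFunction only hides the component passed to it.
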(event OnClicked(m_tileMesh)
  (params (TouchedComponent :type Primitive%20Component%20Object%20Reference) (ButtonPressed :type Key%20Structure :default "None"))
  (Class|HexTile|HexClicked))

(event EventBeginPlay
  (Rendering|SetVisibility (Variables|Default|Getm_tileHighlight) false false)
  (Rendering|SetVisibility (Variables|Default|Getm_tileAttackHighlight) false false)
  (Rendering|SetVisibility (Variables|Default|Getm_tileSelectHighlight) false false)
  (Rendering|SetVisibility (Variables|Default|Getm_tileAttackSelectHighlight) false false))

(event Collision|EventActorBeginOverlap
  (params (OtherActor :type Actor%20Object%20Reference)))

(event EventTick
  (params (DeltaSeconds :type Float%20%28single-precision%29)))

(fn ConstructionScript)

(fn NewFunction
  (params (self2 :type Scene%20Component%20Object%20Reference))
  (Rendering|SetVisibility self2 false false))